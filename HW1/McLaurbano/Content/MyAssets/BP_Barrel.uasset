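; BP_Barrel is a shootable target barrel with a floating health bar that turns each tick to face the player camera.
; Hits from BP_FirstPersonProjectile lower Health in fixed steps and push the value to its Enemy_Health_Bar widget.
; A hit at the last step reveals the fire effect, hides the bar and, through a DoOnce, increments the player character's TargetsEliminated count.
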(event EventTick
  (params (DeltaSeconds :type Float%20%28single-precision%29))
  ;[1 1 1] Rotate Health Bar to Always Face the Player
  (Transformation|SetWorldRotation (Variables|Default|GetWidget) (Math|Rotator|FindLookatRotation (Transformation|GetWorldLocation (Variables|Default|GetWidget)) (Transformation|GetWorldLocation (Variables|/Script/Engine.PlayerCameraManager|GetTransformComponent (Game|GetPlayerCameraManager 0)))) false false))

(event Collision|EventHit
  (params (MyComp :type Primitive%20Component%20Object%20Reference) (Other :type Actor%20Object%20Reference) (OtherComp :type Primitive%20Component%20Object%20Reference) (bSelfMoved :type Boolean) (HitLocation :type Vector :default "0, 0, 0") (HitNormal :type Vector :default "0, 0, 0") (NormalImpulse :type Vector :default "0, 0, 0") (Hit :type Hit%20Result%20Structure%20%28by%20ref%29))
  ;[1 1 1] Update Health, Display Fire and Destroy Health Bar at 0 Health and Update UI Elements
  (Utilities|Casting|CastToBP_FirstPersonProjectile Other)
  (if (<= (Variables|Default|GetHealth) 1e+01)
    (Development|SetHiddeninGame (Variables|/Game/StarterContent/Blueprints/Blueprint_Effect_Fire.Blueprint_Effect_Fire_C|GetP_Fire (Variables|Default|GetFireEffect)) false false)
    (Development|SetHiddeninGame (Variables|Default|GetWidget) true false)
    ;[1 1 1] Update Targets Remaining UI
    (bind _asbp_first_person_character (Utilities|Casting|CastToBP_FirstPersonCharacter (Game|GetPlayerCharacter 0)))
    (Utilities|FlowControl|DoOnce false
      (:Completed
        (bind _result (Math|Integer|IncrementInt (Variables|/Game/FirstPerson/Blueprints/BP_FirstPersonCharacter.BP_FirstPersonCharacter_C|GetTargetsEliminated _asbp_first_person_character))
          (:%20%20
            (Variables|/Game/FirstPerson/Blueprints/BP_FirstPersonCharacter.BP_FirstPersonCharacter_C|SetTargetsEliminated _asbp_first_person_character _result)))))
    (else
      (Variables|Default|SetHealth (- (Variables|Default|GetHealth) 1e+01))
      (bind _asenemy_health_bar (Utilities|Casting|CastToEnemy_Health_Bar (UserInterface|GetWidget (Variables|Default|GetWidget))))
      (Default|UpdateHealthBar _asenemy_health_bar (Variables|Default|GetHealth)))))

(fn ConstructionScript)